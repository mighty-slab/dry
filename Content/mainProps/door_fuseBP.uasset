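; Door fuse prop that the player carries and installs into a door's fusebox.
; On interact, it searches overlapping actors for a doorBP tagged "door" and snaps onto the first socket of that door's DoorFusebox.
; It then plays a sound, notifies the door via GotFused, flags itself as picked up and empties the player's right or left hand.
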(event Custom|interact
  (params (RHand? :type Boolean) (playerRef :type BP%20First%20Person%20Character%20Object%20Reference))
  (bind _empty (Variables|Default|Getempty))
  (bind _array_element (Utilities|Array|ForEachLoopwithBreak (Collision|GetOverlappingActors 0 :!class /Script/Engine.Actor) :!label _label)
    (:LoopBody
      (if (Actor|ActorHasTag _array_element "door")
        (bind _asdoor_bp (Utilities|Casting|CastTodoorBP _array_element))
        (bind _array_element_2 (Utilities|Array|ForEachLoopwithBreak (Transformation|GetAllSocketNames (Variables|/Game/mainProps/doorBP.doorBP_C|Getdoor_fusebox _asdoor_bp)))
          (:LoopBody
            (Transformation|AttachComponentToComponent (Variables|/Game/mainProps/doorBP.doorBP_C|Getdoor_fusebox _asdoor_bp) _array_element_2 "SnapToTarget" "SnapToTarget" "SnapToTarget" true)
            (Audio|Components|Audio|Play (Variables|Default|GetplaceCrankTemp_0) 0.0)
            (Default|GotFused _asdoor_bp)
            (Variables|Default|SetisPickedup true)
            (if RHand?
              (Variables|/Game/FirstPerson/Blueprints/BP_FirstPersonCharacter.BP_FirstPersonCharacter_C|SetheldItem_r playerRef _empty)
              (Variables|/Game/FirstPerson/Blueprints/BP_FirstPersonCharacter.BP_FirstPersonCharacter_C|SetisHolding_r playerRef false)
              (goto _label Break)
              (else
                (Variables|/Game/FirstPerson/Blueprints/BP_FirstPersonCharacter.BP_FirstPersonCharacter_C|SetheldItem_l playerRef _empty)
                (Variables|/Game/FirstPerson/Blueprints/BP_FirstPersonCharacter.BP_FirstPersonCharacter_C|SetisHolding_l playerRef false)
                (goto _label Break)))))))))

(event EventBeginPlay)

(event Collision|EventActorBeginOverlap
  (params (OtherActor :type Actor%20Object%20Reference)))

(event EventTick
  (params (DeltaSeconds :type Float%20%28single-precision%29)))

(fn ConstructionScript)