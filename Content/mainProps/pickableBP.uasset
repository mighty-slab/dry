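; Base pickable prop that the player can carry in either hand and drop, simulating physics while loose.
; Separate left and right attach events play a pickup sound, disable physics and pickup overlaps, and snap it to a socket on the first-person mesh.
; Dropping plays a sound, detaches it in place and restores physics and overlaps.
; Interact is a stub that returns false.
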(event Custom|attachToPlayer_r
  (params (playerReference :type BP%20First%20Person%20Character%20Object%20Reference))
  (Audio|Components|Audio|Play (Variables|Default|GetpickUpsound) 0.0)
  (Variables|Default|SetisPickedup true)
  (Physics|SetSimulatePhysics (Variables|Default|GetStaticMesh) false)
  (Variables|/Script/Engine.PrimitiveComponent|SetbGenerateOverlapEvents (Variables|Default|GetpickUpArea) false)
  (Transformation|AttachComponentToComponent (Variables|/Game/FirstPerson/Blueprints/BP_FirstPersonCharacter.BP_FirstPersonCharacter_C|GetFirstPersonMesh playerReference) "rootSocket" "SnapToTarget" "SnapToTarget" "SnapToTarget" true))

(event Custom|dropFromPlayer
  (params (playerReference :type BP%20First%20Person%20Character%20Object%20Reference))
  (Audio|Components|Audio|Play (Variables|Default|GetdropSound) 0.0)
  (Variables|Default|SetisPickedup false)
  (Variables|/Script/Engine.PrimitiveComponent|SetbGenerateOverlapEvents (Variables|Default|GetpickUpArea) true)
  (Transformation|DetachFromActor "KeepWorld" "KeepWorld" "KeepWorld")
  (Physics|SetSimulatePhysics (Variables|Default|GetStaticMesh) true))

(event Custom|attachToPlayer_l
  (params (playerReference :type BP%20First%20Person%20Character%20Object%20Reference))
  (Audio|Components|Audio|Play (Variables|Default|GetpickUpsound) 0.0)
  (Variables|Default|SetisPickedup true)
  (Physics|SetSimulatePhysics (Variables|Default|GetStaticMesh) false)
  (Variables|/Script/Engine.PrimitiveComponent|SetbGenerateOverlapEvents (Variables|Default|GetpickUpArea) false)
  (Transformation|AttachComponentToComponent (Variables|/Game/FirstPerson/Blueprints/BP_FirstPersonCharacter.BP_FirstPersonCharacter_C|GetFirstPersonMesh playerReference) "rootSocket_0" "SnapToTarget" "SnapToTarget" "SnapToTarget" true))

(event EventBeginPlay
  (Physics|SetSimulatePhysics (Variables|Default|GetStaticMesh) true))

(event Collision|EventActorBeginOverlap
  (params (OtherActor :type Actor%20Object%20Reference)))

(event EventTick
  (params (DeltaSeconds :type Float%20%28single-precision%29)))

(fn ConstructionScript)

(fn Interact
  (params (player :type BP%20First%20Person%20Character%20Object%20Reference) (r_hand? :type Boolean))
  (return false))