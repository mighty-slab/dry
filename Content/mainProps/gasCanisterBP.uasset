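; Interactable gas canister that carries fuel from a gas nozzle to the car to progress the game.
; Interacting checks overlapping actors by tag: a nozzle gets used and, if cranked with capacity left, fills the canister, swaps its material and attaches a spawned TargetPoint.
; At a car, a filled canister empties, restores its material and increments the car's refill count.
; The third refill recolors the car and opens the rigOpen level.
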(event Custom|use
  (params (RHand? :type Boolean) (playerRef :type BP%20First%20Person%20Character%20Object%20Reference))
  (bind _array_element (Utilities|Array|ForEachLoopwithBreak (Collision|GetOverlappingActors 0 :!class /Script/Engine.Actor))
    (:LoopBody
      (if (Actor|ActorHasTag _array_element "nozzle")
        (bind _asgas_nozzle_bp (Utilities|Casting|CastTogasNozzleBP _array_element))
        (Default|GotUsed _asgas_nozzle_bp)
        (if (and (!= (Variables|/Game/mainProps/gasNozzleBP.gasNozzleBP_C|Getcapacity _asgas_nozzle_bp) 0) (Variables|/Game/mainProps/gasNozzleBP.gasNozzleBP_C|GetisCranked _asgas_nozzle_bp))
          (Variables|Default|SetisFilled true)
          (Rendering|Material|SetMaterial (Variables|Default|GetStaticMesh) 0 "/Game/mainProps/meshes/nozzle/nozzleMat.nozzleMat")
          (bind _returnvalue (Game|SpawnActorfromClass "/Script/Engine.TargetPoint" (Transformation|GetActorTransform self) "Undefined" 0 0))
          (Transformation|AttachActorToActor _returnvalue self "None" "SnapToTarget" "SnapToTarget" "SnapToTarget" true))
        (elif (Actor|ActorHasTag _array_element "car")
          (bind _ascar_blueprint (Utilities|Casting|CastTocar_Blueprint _array_element))
          (if (Variables|Default|GetisFilled)
            (bind _output_get (Variables|/Game/mainProps/meshes/car/car_Blueprint.car_Blueprint_C|Setrefills _ascar_blueprint (+ (Variables|/Game/mainProps/meshes/car/car_Blueprint.car_Blueprint_C|Getrefills _ascar_blueprint) 1)))
            (Variables|Default|SetisFilled false)
            (Rendering|Material|SetMaterial (Variables|Default|GetStaticMesh) 0 "/Game/FPWeapon/Materials/BaseMaterial.BaseMaterial")
            (if (== _output_get 3)
              (Rendering|Material|SetMaterial (Variables|/Script/Engine.StaticMeshActor|GetStaticMeshComponent _ascar_blueprint) 0 "/Game/mainProps/meshes/nozzle/nozzleMat.nozzleMat")
              (if (== (Variables|/Game/mainProps/meshes/car/car_Blueprint.car_Blueprint_C|Getrefills _ascar_blueprint) 3)
                (Game|OpenLevel(byName) "rigOpen")))))))))

(event EventTick
  (params (DeltaSeconds :type Float%20%28single-precision%29)))

(fn ConstructionScript)

(fn Interact
  (params (player :type BP%20First%20Person%20Character%20Object%20Reference) (r_hand? :type Boolean))
  (CallFunction|Use r_hand? player)
  (return true))