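; Refillable lantern that lights up brightly for a limited time when refilled from a gas nozzle.
; Interact calls refill, which finds an overlapping "nozzle" actor, calls its GotUsed, then requires it to be cranked with non-zero capacity.
; Success boosts the point light, disables mesh shadows and starts the hum until a LightTime delay ends.
; BeginPlay shares that reset path, so the lantern starts dim and unfilled.
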(event Custom|refill
  (params (RHand? :type Boolean) (playerRef :type BP%20First%20Person%20Character%20Object%20Reference))
  (bind _array_element (Utilities|Array|ForEachLoopwithBreak (Collision|GetOverlappingActors 0 :!class /Script/Engine.Actor) :!label _label)
    (:LoopBody
      (if (Actor|ActorHasTag _array_element "nozzle")
        (bind _asgas_nozzle_bp (Utilities|Casting|CastTogasNozzleBP _array_element))
        (Default|GotUsed _asgas_nozzle_bp)
        (if (and (!= (Variables|/Game/mainProps/gasNozzleBP.gasNozzleBP_C|Getcapacity _asgas_nozzle_bp) 0) (Variables|/Game/mainProps/gasNozzleBP.gasNozzleBP_C|GetisCranked _asgas_nozzle_bp))
          (Variables|Default|SetisFilled_0 true)
          (Rendering|SetCastShadow (Variables|Default|GetStaticMesh) false)
          (Rendering|Components|Light|SetIntensity (Variables|Default|GetPointLight) 1e+05)
          (Components|Activation|Activate (Variables|Default|GetlightHum) false)
          (Utilities|FlowControl|Delay (Math|Conversions|ToFloat(Integer) (Variables|Default|GetlightTime)))
          (Variables|Default|SetisFilled_0 false)
          (Rendering|SetCastShadow (Variables|Default|GetStaticMesh) true)
          (Rendering|Components|Light|SetIntensity (Variables|Default|GetPointLight) 1e+02)
          (Components|Activation|Deactivate (Variables|Default|GetlightHum))
          (goto _label Break))))))

(event EventBeginPlay
  (Variables|Default|SetisFilled_0 false)
  (Rendering|SetCastShadow (Variables|Default|GetStaticMesh) true)
  (Rendering|Components|Light|SetIntensity (Variables|Default|GetPointLight) 1e+02)
  (Components|Activation|Deactivate (Variables|Default|GetlightHum))
  (Utilities|Array|ForEachLoopwithBreak (Collision|GetOverlappingActors 0 :!class /Script/Engine.Actor)) ; enters at Break
)

(event Collision|EventActorBeginOverlap
  (params (OtherActor :type Actor%20Object%20Reference)))

(fn ConstructionScript)

(fn Interact
  (params (player :type BP%20First%20Person%20Character%20Object%20Reference) (r_hand? :type Boolean))
  (CallFunction|Refill r_hand? player)
  (return true))

(fn IsInteractable?
  (params (other_actor :type Actor%20Object%20Reference))
  (return (Actor|ActorHasTag other_actor "nozzle")))