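; Patrol AI character that walks between two target points, roams, or chases and damages the player.
; BeginPlay picks the starting behavior, and PawnSensing switches to Chase on seeing a player-controlled pawn.
; AIMoveTo callbacks drive self-repeating events: failed chases fall back to Roam, failed roams to Patrol.
; On reaching the player, Chase updates a DamageBox overlap flag, applies damage without branching on it, then repeats after a delay.
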(event OnSeePawn(PawnSensing)
  (params (Pawn :type Pawn%20Object%20Reference))
  ;[1 1 1] OnSeePawn(Checks if Pawn is Player)
  (if (Pawn|IsPlayerControlled Pawn) ; If true, chase
    (Variables|Default|SetInRange? true)
    (CallFunction|Chase)))

(event Custom|Chase
  (bind _returnvalue (Game|GetPlayerCharacter 0))
  ;[1 1 1] Chase Player(Can be any actor as target)
  (CallFunction|StartSprint)
  (AI|AIMoveTo self "0, 0, 0" _returnvalue 5.0 false
    (:then
      (Variables|Default|SetMoving? true) ; Sets Moving to true until AI succesfully reaches Player
    )
    (:OnSuccess
      (CallFunction|CheckPlayerIsinDamageRange) ; This function serves to double check if player is in front of AI. Check inside function for more details
      (Game|Damage|ApplyDamage _returnvalue (Variables|Default|GetBaseDamage) 0 0) ; Damages PlayerCharacter
      (Utilities|FlowControl|Delay 3.0) ; Adding this delay prevents player from constantly taking damage when in damage range
      (CallFunction|Chase))
    (:OnFail
      (CallFunction|Roam) ; Will begin to roam if it can no longer see the player
    )))

(event Custom|Roam
  ;[1 1 1] Roam(Set to random location)
  (CallFunction|StopSprint)
  (Variables|/Script/Engine.CharacterMovementComponent|SetMaxWalkSpeed (Variables|Character|GetCharacterMovement) (* (Variables|Default|GetSprintSpeed) 0.8))
  (AI|AIMoveTo self (.RandomLocation (Class|NavigationSystemV1|GetRandomPointinNavigableRadius (Transformation|GetActorLocation) 5e+02 0 0)) 0 5.0 false
    (:then
      (Variables|Default|SetMoving? true) ; Sets Moving to true until AI succesfully reaches Player
    )
    (:OnSuccess
      (CallFunction|Roam))
    (:OnFail
      (CallFunction|Patrol))))

(event Custom|Patrol
  (bind _self self)
  ;[1 1 1] Patrol(Set to repeat by default)
  (CallFunction|StopSprint) ; Sets AI to walking speed
  (AI|AIMoveTo _self "0, 0, 0" (Variables|Default|GetTargetPoint1) 5.0 false
    (:OnSuccess
      (Utilities|FlowControl|Delay 5.0) ; Duration between moving to next point
      (AI|AIMoveTo _self "0, 0, 0" (Variables|Default|GetTargetPoint2) 5.0 false
        (:OnSuccess
          (Utilities|FlowControl|Delay 5.0) ; Duration between moving to next point
          (CallFunction|Patrol) ; Repeat path
        )))))

(event EventBeginPlay
  ;[1 1 1] BeginPlay(Set default state here)
  (switch Utilities|FlowControl|Switch|SwitchonAI_State "NewEnumerator3"
    (:NewEnumerator1
      (CallFunction|Roam))
    (:NewEnumerator2
      (CallFunction|Chase))
    (:NewEnumerator3
      (CallFunction|Patrol))))

(fn ConstructionScript)

(fn StartSprint
  (Variables|/Script/Engine.CharacterMovementComponent|SetMaxWalkSpeed (Variables|Character|GetCharacterMovement) (Variables|Default|GetSprintSpeed)))

(fn StopSprint
  (Variables|/Script/Engine.CharacterMovementComponent|SetMaxWalkSpeed (Variables|Character|GetCharacterMovement) (Variables|Default|GetWalk%20Speed)))

(fn CheckPlayerIsinDamageRange
  (bind _asplayer_character_bp (Utilities|Casting|CastToPlayerCharacter_BP (Game|GetPlayerCharacter 0))) ; This function only works for checking if demo PlayerCharacter is in DamageBox but can be changed/copied to check for other actors/characters as well
  (if (Collision|IsOverlappingActor (Variables|Default|GetDamageBox) _asplayer_character_bp :!class /Script/Engine.PrimitiveComponent)
    (Variables|Default|SetPlayerIsInDamageRange? true)
    (else
      (Variables|Default|SetPlayerIsInDamageRange? false)))
  (return))